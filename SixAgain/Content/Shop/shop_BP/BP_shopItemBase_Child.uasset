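; Shop item child Blueprint of a base shop item, representing one rarity tier with a blue glow colour.
; On BeginPlay it runs the parent logic, sets Rarity, then creates a dynamic M_shopGlow material instance and tints its GlowColour translucent blue.
; The graph does not assign that material instance to any component.
; AddEffect and the construction script only call the parent, and Tick and overlap are disabled.
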(event EventBeginPlay
  (|CallParentFunction)
  (Variables|Default|SetRarity "NewEnumerator2")
  (bind _returnvalue (Rendering|Material|CreateDynamicMaterialInstance "/Game/particles/ShopGlow/M_shopGlow.M_shopGlow" "None" "None" :!class /Script/Engine.KismetMaterialLibrary))
  (Rendering|Material|SetVectorParameterValue _returnvalue "GlowColour" "(R=0.000000,G=0.057762,B=1.000000,A=0.200000)" :!class /Script/Engine.MaterialInstanceDynamic))

(event Collision|EventActorBeginOverlap
  (params (OtherActor :type Actor%20Object%20Reference))
  (|CallParentFunction OtherActor) ; This node is disabled and will not be called.\nDrag off pins to build functionality.
)

(event EventTick
  (params (DeltaSeconds :type Float%20%28single-precision%29))
  (|CallParentFunction DeltaSeconds) ; This node is disabled and will not be called.\nDrag off pins to build functionality.
)

(fn ConstructionScript
  (|CallParentFunction))

(fn AddEffect
  (|CallParentFunction))