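; BP_shopItemBase is a base shop item that the player buys by interacting with it.
; PlayerInteract casts the player to BP_FirstPersonCharacter_prototype, stores the reference, and deducts Cost from its Money if affordable.
; A successful purchase then calls AddEffect, a placeholder that only prints a debug string in this base.
; The item does nothing when funds are short and is not removed after purchase.
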(event EventBeginPlay)

(event Collision|EventActorBeginOverlap
  (params (OtherActor :type Actor%20Object%20Reference)))

(event EventTick
  (params (DeltaSeconds :type Float%20%28single-precision%29)))

(event EventPlayerInteract
  (params (Player :type Object%20Object%20Reference))
  (bind _asbp_first_person_character_prototype (Utilities|Casting|CastToBP_FirstPersonCharacter_prototype Player))
  (Variables|Default|SetCharater%20Refrence _asbp_first_person_character_prototype)
  (if (>= (Variables|/Game/FirstPerson/Blueprints/BP_FirstPersonCharacter_prototype.BP_FirstPersonCharacter_prototype_C|GetMoney _asbp_first_person_character_prototype) (Variables|Default|GetCost))
    (Variables|/Game/FirstPerson/Blueprints/BP_FirstPersonCharacter_prototype.BP_FirstPersonCharacter_prototype_C|SetMoney (Variables|Default|GetCharater%20Refrence) (- (Variables|/Game/FirstPerson/Blueprints/BP_FirstPersonCharacter_prototype.BP_FirstPersonCharacter_prototype_C|GetMoney (Variables|Default|GetCharater%20Refrence)) (Variables|Default|GetCost)))
    (CallFunction|AddEffect)))

(fn ConstructionScript)

(fn AddEffect
  (Development|PrintString "Base Pick Up"))