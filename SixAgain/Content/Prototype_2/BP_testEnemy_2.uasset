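; Prototype enemy that chases the player once pawn sensing spots a pawn and takes hits reported through HitbyPlayer.
; Head hits deal double damage and higher points, and every hit adds points to the player character's Money and plays a pain sound.
; At zero health it disables movement and collision, then a timeline sinks and pitches it before notifying its home BP_testEnemySpawner and destroying itself.
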(event OnSeePawn(PawnSensing)
  (params (Pawn :type Pawn%20Object%20Reference))
  (CallFunction|FollowPlayer))

(event Custom|FollowPlayer
  (AI|AIMoveTo self "0, 0, 0" (Game|Player|GetPlayerPawn 0) 5.0 false))

(event Custom|PlayPainNoise
  (bind _returnvalue (AddComponent|AddAudioComponent false))
  (Audio|Components|Audio|Play _returnvalue 0.5))

(event EventHitbyPlayer
  (params (HitArea :type Object%20Object%20Reference) (Damage :type Float%20%28double-precision%29))
  (bind _returnvalue (Transformation|GetActorLocation))
  (bind _returnvalue_2 (Transformation|GetActorRotation))
  (if (Utilities|Enum|Equal(Enum) (Utilities|GetObjectName HitArea) "head")
    (Variables|Default|SetPointValue 100)
    (Variables|Default|SetHealth (- (Variables|Default|GetHealth) (* Damage 2.0)))
    (else
      (Variables|Default|SetPointValue 50)
      (Variables|Default|SetHealth (- (Variables|Default|GetHealth) Damage))))
  (CallFunction|GivePoints)
  (CallFunction|PlayPainNoise)
  (if (<= (Variables|Default|GetHealth) 0.0)
    (Pawn|Components|CharacterMovement|DisableMovement (Variables|Character|GetCharacterMovement))
    (Collision|SetCollisionEnabled (Variables|Default|Gethead) "NoCollision")
    (Collision|SetCollisionEnabled (Variables|Default|Getbody) "NoCollision")
    (Collision|SetCollisionEnabled (Variables|Collision|GetCapsuleComponent) "NoCollision")
    (bind (_direction _rotation _down) (Timeline|testEnemyDie Play)
      (:Update
        (Transformation|SetActorLocationAndRotation (Math|Vector|MakeVector (.x _returnvalue) (.y _returnvalue) (- (.z _returnvalue) _down)) (Math|Rotator|MakeRotator (.roll _returnvalue_2) _rotation (.yaw _returnvalue_2))))
      (:Finished
        (bind _asbp_test_enemy_spawner (Utilities|Casting|CastToBP_testEnemySpawner (Variables|Default|GetHomeSpawner)))
        (Default|EnemyDied _asbp_test_enemy_spawner)
        (Actor|DestroyActor)))))

(event EventGivePoints
  (bind _asbp_first_person_character_prototype (Utilities|Casting|CastToBP_FirstPersonCharacter_prototype (Game|Player|GetPlayerPawn 0)))
  (Variables|/Game/FirstPerson/Blueprints/BP_FirstPersonCharacter_prototype.BP_FirstPersonCharacter_prototype_C|SetMoney _asbp_first_person_character_prototype (+ (Variables|/Game/FirstPerson/Blueprints/BP_FirstPersonCharacter_prototype.BP_FirstPersonCharacter_prototype_C|GetMoney _asbp_first_person_character_prototype) (Variables|Default|GetPointValue))))

(fn ConstructionScript)

(fn PlayHurtSound)