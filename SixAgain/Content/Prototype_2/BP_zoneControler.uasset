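; BP_zoneControler is a box-volume zone that unlocks the zombie spawners inside it once the player is present.
; On BeginPlay it caches overlapping BP_zombieSpawner actors, then after a short delay unlocks them if the player starts inside.
; A DoOnce on box overlap, reset for non-player actors, marks the spawners available and has the player's child-actor BP_WaveControler recheck spawners.
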(event OnComponentBeginOverlap(Box)
  (params (OverlappedComponent :type Primitive%20Component%20Object%20Reference) (OtherActor :type Actor%20Object%20Reference) (OtherComp :type Primitive%20Component%20Object%20Reference) (OtherBodyIndex :type Integer) (bFromSweep :type Boolean) (SweepResult :type Hit%20Result%20Structure%20%28by%20ref%29))
  (Utilities|FlowControl|DoOnce false :!label _label
    (:Completed
      (bind _asbp_first_person_character_prototype (Utilities|Casting|CastToBP_FirstPersonCharacter_prototype OtherActor)
        (:then
          (CallFunction|UnlockArea)
          (bind _asbp_wave_controler (Utilities|Casting|CastToBP_WaveControler (Variables|/Script/Engine.ChildActorComponent|GetChildActor (Variables|/Game/FirstPerson/Blueprints/BP_FirstPersonCharacter_prototype.BP_FirstPersonCharacter_prototype_C|GetWaveController _asbp_first_person_character_prototype))))
          (Default|RecheckSpawner _asbp_wave_controler))
        (:CastFailed
          (goto _label Reset))))))

(event Custom|UnlockArea
  (for _array_element (Variables|Default|GetZoneSpawners)
    (bind _asbp_zombie_spawner (Utilities|Casting|CastToBP_zombieSpawner _array_element))
    (Variables|/Game/Prototype_2/BP_zombieSpawner.BP_zombieSpawner_C|SetIsAvailable? _asbp_zombie_spawner true))
  (Development|PrintString "Area Unlocked"))

(event EventBeginPlay
  (bind _output_get (Variables|Default|SetZoneSpawners (Collision|GetOverlappingActors (Variables|Default|GetBox) "/Game/Prototype_2/BP_zombieSpawner.BP_zombieSpawner_C" :!class /Script/Engine.PrimitiveComponent)))
  (Development|PrintString (Utilities|GetDisplayName (.OutItem (Utilities|Array|Random _output_get))))
  (Utilities|FlowControl|Delay 0.2)
  (Utilities|Casting|CastToBP_FirstPersonCharacter_prototype (.OutItem (Utilities|Array|Random (Collision|GetOverlappingActors (Variables|Default|GetBox) "/Game/FirstPerson/Blueprints/BP_FirstPersonCharacter_prototype.BP_FirstPersonCharacter_prototype_C" :!class /Script/Engine.PrimitiveComponent))))
  (CallFunction|UnlockArea))

(event Collision|EventActorBeginOverlap
  (params (OtherActor :type Actor%20Object%20Reference)))

(event EventTick
  (params (DeltaSeconds :type Float%20%28single-precision%29)))

(fn ConstructionScript)