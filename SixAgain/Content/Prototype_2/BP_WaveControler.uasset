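; BP_WaveControler is a prototype wave controller that tracks wave number and spawn budget and toggles distance-triggered objects.
; A sphere overlap calls ToggleActive on BPI_DistanceTriggered actors entering or leaving it, keeping them in ActiveObjects.
; Tick calls ProgressWave whenever SpawnBudget is above zero, raising the wave and refilling a growing budget.
; Nothing here spends the budget or spawns, so waves advance every frame while it stays positive.
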(event OnComponentBeginOverlap(Sphere)
  (params (OverlappedComponent :type Primitive%20Component%20Object%20Reference) (OtherActor :type Actor%20Object%20Reference) (OtherComp :type Primitive%20Component%20Object%20Reference) (OtherBodyIndex :type Integer) (bFromSweep :type Boolean) (SweepResult :type Hit%20Result%20Structure%20%28by%20ref%29))
  (bind _asbpi_distance_triggered (Utilities|Casting|CastToBPI_DistanceTriggered OtherActor))
  (Default|ToggleActive _asbpi_distance_triggered)
  (Utilities|Array|Add (Variables|Default|GetActiveObjects) OtherActor))

(event OnComponentEndOverlap(Sphere)
  (params (OverlappedComponent :type Primitive%20Component%20Object%20Reference) (OtherActor :type Actor%20Object%20Reference) (OtherComp :type Primitive%20Component%20Object%20Reference) (OtherBodyIndex :type Integer))
  (bind _asbpi_distance_triggered (Utilities|Casting|CastToBPI_DistanceTriggered OtherActor))
  (Default|ToggleActive _asbpi_distance_triggered)
  (Utilities|Array|RemoveItem (Variables|Default|GetActiveObjects) OtherActor))

(event EventBeginPlay
  (Variables|Default|SetWave 1)
  (Variables|Default|SetSpawnBudget (Variables|Default|GetTotalWaveSpawnBudget)))

(event Collision|EventActorBeginOverlap
  (params (OtherActor :type Actor%20Object%20Reference)))

(event EventTick
  (params (DeltaSeconds :type Float%20%28single-precision%29))
  (if (> (Variables|Default|GetSpawnBudget) 0)
    (CallFunction|ProgressWave)))

(fn ConstructionScript)

(fn ProgressWave
  (Variables|Default|SetWave (+ (Variables|Default|GetWave) 1))
  (bind _output_get (Variables|Default|SetTotalWaveSpawnBudget (+ (Variables|Default|GetTotalWaveSpawnBudget) 3)))
  (Variables|Default|SetSpawnBudget _output_get))