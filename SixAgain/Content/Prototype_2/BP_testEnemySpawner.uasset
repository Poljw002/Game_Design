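; Prototype enemy spawner that keeps a population of BP_Spider_Zombie actors topped up to MaxSpawned.
; Tick checks CurrentSpawned against the cap and swaps the Sphere's material between go and stop indicators.
; Below the cap, a two-second Delay on Tick paces spawns at SpawnPlate's location and rotation, incrementing the count.
; Each zombie receives this spawner as HomeSpawner, and the EnemyDied event decrements the count to free a slot.
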(event Custom|Enemy%20Died
  (Variables|Default|SetCurrentSpawned (- (Variables|Default|GetCurrentSpawned) 1)))

(event EventTick
  (params (DeltaSeconds :type Float%20%28single-precision%29))
  (bind _spawnplate (Variables|Default|GetSpawnPlate))
  (bind _returnvalue (Transformation|GetWorldTransform _spawnplate))
  (if (< (Variables|Default|GetCurrentSpawned) (Variables|Default|GetMaxSpawned))
    (Rendering|Material|SetMaterial (Variables|Default|GetSphere) 0 "/Game/Prototype_2/testMats/M_SpawnIndicator_go.M_SpawnIndicator_go")
    (Utilities|FlowControl|Delay 2.0)
    (Game|SpawnActorfromClass "/Game/NPCs/Basic_Zombie/BP_Spider_Zombie.BP_Spider_Zombie_C" (Math|Transform|MakeTransform (.location _returnvalue) (.rotation _returnvalue) "1.000000,1.000000,1.000000") "Undefined" "MultiplyWithRoot" 0 self 0)
    (Variables|Default|SetCurrentSpawned (+ (Variables|Default|GetCurrentSpawned) 1))
    (else
      (Rendering|Material|SetMaterial (Variables|Default|GetSphere) 0 "/Game/Prototype_2/testMats/M_SpawnIndicator_Stop.M_SpawnIndicator_Stop"))))

(fn ConstructionScript)