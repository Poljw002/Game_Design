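; Spider zombie enemy that chases the player by re-issuing AI MoveTo every Tick; pawn sensing only calls an empty FollowPlayer event.
; Hits double damage on the head collision, add money to the player and play a pain sound.
; At zero health it ragdolls, notifies its spawner and is destroyed after a delay.
; Capsule resizing and timeline death animation are unwired, and several functions are empty stubs.
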(event OnSeePawn(PawnSensing)
  (params (Pawn :type Pawn%20Object%20Reference))
  (CallFunction|FollowPlayer))

(event Custom|FollowPlayer)

(event Custom|PlayPainNoise
  (bind _returnvalue (AddComponent|AddAudioComponent false))
  (Audio|Components|Audio|Play _returnvalue 0.5))

(event EventTick
  (params (DeltaSeconds :type Float%20%28single-precision%29))
  (AI|AIMoveTo self "0, 0, 0" (Game|Player|GetPlayerPawn 0) 5.0 false))

(event EventHitbyPlayer
  (params (HitArea :type Object%20Object%20Reference) (Damage :type Float%20%28double-precision%29))
  (bind _mesh (Variables|Character|GetMesh))
  (CallFunction|CalculateDamageTaken Damage HitArea)
  (CallFunction|GivePoints)
  (CallFunction|PlayPainNoise)
  (if (<= (Variables|Default|GetHealth) 0.0)
    (Pawn|Components|CharacterMovement|DisableMovement (Variables|Character|GetCharacterMovement))
    (Collision|SetCollisionProfileName _mesh "Ragdoll" true :!class /Script/Engine.PrimitiveComponent)
    (Physics|SetSimulatePhysics _mesh true)
    (bind _asbp_test_enemy_spawner (Utilities|Casting|CastToBP_testEnemySpawner (Variables|Default|GetHomeSpawner))
      (:then
        (Default|EnemyDied _asbp_test_enemy_spawner))
      (:CastFailed
        _))
    (Utilities|FlowControl|Delay 3.0)
    (Actor|DestroyActor)))

(event EventGivePoints
  (bind _asbp_first_person_character_prototype (Utilities|Casting|CastToBP_FirstPersonCharacter_prototype (Game|Player|GetPlayerPawn 0)))
  (Variables|/Game/FirstPerson/Blueprints/BP_FirstPersonCharacter_prototype.BP_FirstPersonCharacter_prototype_C|SetMoney _asbp_first_person_character_prototype (+ (Variables|/Game/FirstPerson/Blueprints/BP_FirstPersonCharacter_prototype.BP_FirstPersonCharacter_prototype_C|GetMoney _asbp_first_person_character_prototype) (Variables|Default|GetPointValue))))

(fn ConstructionScript)

(fn PlayHurtSound)

(fn CalculateDamageTaken
  (params (RawDamage :type Float%20%28double-precision%29) (HitZone :type Object%20Object%20Reference))
  (if (Utilities|Enum|Equal(Enum) (Utilities|GetObjectName HitZone) "head_collison")
    (Variables|Default|SetHealth (- (Variables|Default|GetHealth) (* RawDamage 2.0)))
    (Variables|Default|SetPointValue 100)
    (else
      (Variables|Default|SetHealth (- (Variables|Default|GetHealth) RawDamage))
      (Variables|Default|SetPointValue 50))))

(fn AwardPoints)

(fn SetCrawl
  (if (Variables|Default|Getcrawling)
    (Variables|Default|Setcrawling false)
    (else
      (Variables|Default|Setcrawling true))))