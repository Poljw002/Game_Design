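; Spider zombie enemy for a wave-based game that chases the player and awards money on each hit.
; Tick drives AIMoveTo; arrival opens a one-second stationary attack window for HurtBox damage, while the pawn-sensing FollowPlayer event is empty.
; HitbyPlayer doubles headshot damage and pays out PointValue, which overwrites the shop's tarot bonus.
; Death ragdolls the mesh, notifies the wave controller and destroys the actor after a delay.
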(event OnSeePawn(PawnSensing)
  (params (Pawn :type Pawn%20Object%20Reference))
  (CallFunction|FollowPlayer))

(event OnComponentBeginOverlap(HurtBox)
  (params (OverlappedComponent :type Primitive%20Component%20Object%20Reference) (OtherActor :type Actor%20Object%20Reference) (OtherComp :type Primitive%20Component%20Object%20Reference) (OtherBodyIndex :type Integer) (bFromSweep :type Boolean) (SweepResult :type Hit%20Result%20Structure%20%28by%20ref%29))
  (if (Variables|Default|GetIsAttacking?)
    (bind _asbp_first_person_character_prototype (Utilities|Casting|CastToBP_FirstPersonCharacter_prototype OtherActor))
    (Development|PrintString "OUCH")
    (Default|TakeDamage _asbp_first_person_character_prototype (Variables|Default|GetDamage))))

(event Custom|FollowPlayer)

(event Custom|PlayPainNoise
  (bind _returnvalue (AddComponent|AddAudioComponent false))
  (Audio|Components|Audio|Play _returnvalue 0.5))

(event EventTick
  (params (DeltaSeconds :type Float%20%28single-precision%29))
  (bind _charactermovement (Variables|Character|GetCharacterMovement))
  (AI|AIMoveTo self "0, 0, 0" (Game|Player|GetPlayerPawn 0) 5e+01 false
    (:OnSuccess
      (Variables|Default|SetIsAttacking? true)
      (Pawn|Components|CharacterMovement|DisableMovement _charactermovement)
      (Utilities|FlowControl|Delay 1.0)
      (Variables|Default|SetIsAttacking? false)
      (Pawn|Components|CharacterMovement|SetMovementMode _charactermovement "MOVE_NavWalking" 0))))

(event EventHitbyPlayer
  (params (HitArea :type Object%20Object%20Reference) (Damage :type Float%20%28double-precision%29))
  (bind _mesh (Variables|Character|GetMesh))
  (bind _foundwidgets (Widget|GetAllWidgetsOfClass "/Game/Shop/ShopNew/ShopInterface.ShopInterface_C" true))
  (Variables|Default|SetPointValue (+ (Variables|Default|GetPointValue) (* (Utilities|Array|Get(acopy) (Variables|/Game/Shop/ShopNew/ShopInterface.ShopInterface_C|GetTarotCount (Utilities|Array|Get(acopy) _foundwidgets)) 2) 10)))
  (CallFunction|CalculateDamageTaken Damage HitArea)
  (CallFunction|GivePoints)
  (CallFunction|PlayPainNoise)
  (if (<= (Variables|Default|GetHealth) 0.0)
    (Pawn|Components|CharacterMovement|DisableMovement (Variables|Character|GetCharacterMovement))
    (Collision|SetCollisionEnabled (Variables|Collision|GetCapsuleComponent) "NoCollision")
    (Collision|SetCollisionEnabled (Variables|Default|GetHead_collison) "NoCollision")
    (Collision|SetCollisionEnabled (Variables|Default|GetBody_collider_3) "NoCollision")
    (Collision|SetCollisionProfileName _mesh "Ragdoll" false :!class /Script/Engine.PrimitiveComponent)
    (Physics|SetSimulatePhysics _mesh true)
    (bind _asbp_wave_controler (Utilities|Casting|CastToBP_WaveControler (Variables|Default|GetWaveManager)))
    (Default|EnemyDied _asbp_wave_controler)
    (Utilities|FlowControl|Delay 3.0)
    (Actor|DestroyActor)))

(event EventGivePoints
  (bind _asbp_first_person_character_prototype (Utilities|Casting|CastToBP_FirstPersonCharacter_prototype (Game|Player|GetPlayerPawn 0)))
  (Variables|/Game/FirstPerson/Blueprints/BP_FirstPersonCharacter_prototype.BP_FirstPersonCharacter_prototype_C|SetMoney _asbp_first_person_character_prototype (+ (Variables|/Game/FirstPerson/Blueprints/BP_FirstPersonCharacter_prototype.BP_FirstPersonCharacter_prototype_C|GetMoney _asbp_first_person_character_prototype) (Variables|Default|GetPointValue))))

(fn ConstructionScript)

(fn PlayHurtSound)

(fn CalculateDamageTaken
  (params (RawDamage :type Float%20%28double-precision%29) (HitZone :type Object%20Object%20Reference))
  (if (Utilities|Enum|Equal(Enum) (Utilities|GetObjectName HitZone) "head_collison")
    (Variables|Default|SetHealth (- (Variables|Default|GetHealth) (* RawDamage 2.0)))
    (Variables|Default|SetPointValue 100)
    (else
      (Variables|Default|SetHealth (- (Variables|Default|GetHealth) RawDamage))
      (Variables|Default|SetPointValue 50))))

(fn AwardPoints)

(fn SetCrawl
  (if (Variables|Default|Getcrawling)
    (Variables|Default|Setcrawling false)
    (else
      (Variables|Default|Setcrawling true))))